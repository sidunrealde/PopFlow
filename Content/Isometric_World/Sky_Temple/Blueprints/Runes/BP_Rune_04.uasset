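; BP_Rune_04 is a floating rune in the Sky Temple that acts as a key-gated goal.
; When a Character overlaps its R component, it opens the game mode's congratulations menu if at least three keys are held, otherwise showing the HUD objective.
; Leaving the overlap hides the objective.
; A restarting timeline bobs the mesh, starting at a random time to vary its phase.
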(event OnComponentBeginOverlap(r)
  (params (OverlappedComponent :type Primitive%20Component%20Object%20Reference) (OtherActor :type Actor%20Object%20Reference) (OtherComp :type Primitive%20Component%20Object%20Reference) (OtherBodyIndex :type Integer) (bFromSweep :type Boolean) (SweepResult :type Hit%20Result%20Structure%20%28by%20ref%29))
  (bind _gamemoderef (Variables|Default|GetGameModeRef))
  (Utilities|Casting|CastToCharacter OtherActor)
  (if (>= (Variables|/Game/AdvancedLocomotionV4/Blueprints/GameModes/ALS_GameMode_SP.ALS_GameMode_SP_C|GetKeys (Variables|Default|GetGameModeRef)) 3)
    (Default|CreateCongratulationsMenu _gamemoderef)
    (else
      (bind _hudref (Variables|/Game/AdvancedLocomotionV4/Blueprints/GameModes/ALS_GameMode_SP.ALS_GameMode_SP_C|GetHUDRef _gamemoderef)
        (:then
          (Variables|/Game/PopFlow/Assets/UI/W_HUD.W_HUD_C|SetbShowObjective _hudref true))
        (:else)))))

(event OnComponentEndOverlap(r)
  (params (OverlappedComponent :type Primitive%20Component%20Object%20Reference) (OtherActor :type Actor%20Object%20Reference) (OtherComp :type Primitive%20Component%20Object%20Reference) (OtherBodyIndex :type Integer))
  (Utilities|Casting|CastToCharacter OtherActor)
  (bind _hudref (Variables|/Game/AdvancedLocomotionV4/Blueprints/GameModes/ALS_GameMode_SP.ALS_GameMode_SP_C|GetHUDRef (Variables|Default|GetGameModeRef))
    (:then
      (Variables|/Game/PopFlow/Assets/UI/W_HUD.W_HUD_C|SetbShowObjective _hudref false))
    (:else)))

(event EventBeginPlay
  (bind _asals_game_mode_sp (Utilities|Casting|CastToALS_GameMode_SP (Game|GetGameMode)))
  (Variables|Default|SetGameModeRef _asals_game_mode_sp)
  (Utilities|FlowControl|Sequence
    (:then_1
      (bind _position (Timeline|Timeline_0 SetNewTime)
        (:Update
          (Transformation|SetRelativeLocation (Variables|Default|GetStaticMesh) (* _position "10.000000,0,20.000000") false false))
        (:Finished
          (Utilities|FlowControl|Sequence
            (:then_0
              (Timeline|Timeline_0 PlayFromStart))))))
    (:then_2
      (Timeline|Timeline_0 Play))))

(fn ConstructionScript)