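; BP_BubbleSpawner keeps a floating bubble present in its box volume for the floating bubble puzzle.
; On BeginPlay it spawns a BP_FloatingBubbles at a random point inside the Box component's bounds and plays a pop sound there.
; It binds to that bubble's OnBubbleDestroyed dispatcher, so each destruction spawns the next bubble, chaining one at a time.
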(event Custom|OnBubbleDestroyed_Event
  (CallFunction|SpawnBubble))

(event Custom|SpawnBubble
  (bind _box (Variables|Default|GetBox))
  (bind (_origin _boxextent) (Collision|GetComponentBounds _box))
  (bind _returnvalue (Game|SpawnActorfromClass "/Game/PopFlow/Blueprints/FloatingBubblePuzzle/BP_FloatingBubbles.BP_FloatingBubbles_C" (Math|Transform|MakeTransform (Math|Random|RandomPointinBoundingBox _origin _boxextent) "0, 0, 0" "1.000000,1.000000,1.000000") "Undefined" "MultiplyWithRoot" 0 0))
  (bind _output_get (Variables|Default|SetFloatingBubbleRef _returnvalue))
  (EventDispatchers|AssignOnBubbleDestroyed _output_get (delegate Custom|OnBubbleDestroyed_Event))
  (Audio|PlaySoundatLocation "/Game/Interface_And_Item_Sounds/Cues/Pop_02_Cue.Pop_02_Cue" (Transformation|GetActorLocation _returnvalue) "0, 0, 0" 1.0 1.0 0.0 0 0 0 0))

(event EventBeginPlay
  (CallFunction|SpawnBubble))

(fn ConstructionScript)