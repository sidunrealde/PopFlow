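; BP_BubblePathway is a bubble bridge for the floating bubble puzzle that builds itself progressively along a spline when StartBridge is called.
; StartBridge derives the step count from the spline length and starts a looping timer.
; Each tick adds a pair of instanced meshes at evenly spaced spline distances, offset to either side on local Y rather than following spline rotation.
; Past the last step, it clears the timer and plays a pop sound.
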(event Custom|StartBridge
  (Variables|Default|SetIndex 0)
  (Variables|Default|SetMaxIndex (Math|Float|Truncate (/ (Spline|GetSplineLength (Variables|Default|GetSpline)) 1.5e+02)))
  (bind _returnvalue (Utilities|Time|SetTimerbyEvent (delegate Custom|BubbleBridgeConstruction) 0.2 true))
  (Variables|Default|SetBridgeTimer _returnvalue))

(event Custom|BubbleBridgeConstruction
  (bind _index (Variables|Default|GetIndex))
  (bind _spline (Variables|Default|GetSpline))
  (bind _index_2 (Variables|Default|GetIndex))
  (bind _returnvalue (* _index 150))
  (bind _returnvalue_2 (Math|Conversions|ToFloat(Integer) _returnvalue))
  (bind _returnvalue_3 (Spline|GetLocationatDistanceAlongSpline _spline _returnvalue_2 "Local"))
  (Components|InstancedStaticMesh|AddInstances (Variables|Default|GetInstancedStaticMesh) (Utilities|Array|MakeArray (Math|Transform|MakeTransform (+ _returnvalue_3 "0.000000,75.000000,0.000000") "0, 0, 0" "1.000000,1.000000,1.000000") (Math|Transform|MakeTransform (+ _returnvalue_3 "0.000000,-75.000000,0.000000") "0, 0, 0" "1.000000,1.000000,1.000000")) false false true)
  (Math|Integer|IncrementInt _index_2
    (:%20%20
      (if (> _index_2 (Variables|Default|GetMaxIndex))
        (Utilities|Time|ClearandInvalidateTimerbyHandle (Variables|Default|GetBridgeTimer))
        (Audio|PlaySoundatLocation "/Game/Interface_And_Item_Sounds/Cues/Pop_01_Cue.Pop_01_Cue" (Transformation|GetActorLocation) "0, 0, 0" 1.0 1.0 0.0 0 0 0 0)))))

(fn ConstructionScript)