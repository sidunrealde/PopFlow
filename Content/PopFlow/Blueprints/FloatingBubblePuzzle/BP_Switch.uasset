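; Pressure plate switch for the floating bubble puzzle that drives a referenced fan, moving it forward or back or turning it on, according to SwitchType.
; Pawn or WorldDynamic overlap lights the tile through a dynamic material, plays a clank, lowers it via timeline and triggers the fan.
; Any end overlap or SwitchOff call reverses the tile and glow and stops the fan action, unless ClonePlaced holds it down.
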(event OnComponentBeginOverlap(Box)
  (params (OverlappedComponent :type Primitive%20Component%20Object%20Reference) (OtherActor :type Actor%20Object%20Reference) (OtherComp :type Primitive%20Component%20Object%20Reference) (OtherBodyIndex :type Integer) (bFromSweep :type Boolean) (SweepResult :type Hit%20Result%20Structure%20%28by%20ref%29))
  (bind _returnvalue (Collision|GetCollisionObjectType OtherComp))
  (bind _fanref (Variables|Default|GetFanRef))
  (bind _dynamicmaterial (Variables|Default|GetDynamicMaterial))
  (if (or (Utilities|Enum|Equal(Enum) _returnvalue "ECC_WorldDynamic") (Utilities|Enum|Equal(Enum) _returnvalue "ECC_Pawn"))
    (Rendering|Material|SetScalarParameterValue _dynamicmaterial "SwitchIntensity" 1.0 :!class /Script/Engine.MaterialInstanceDynamic)
    (Rendering|Material|SetMaterial (Variables|Default|GetSM_Temple_Floor_Tile_2m_01) 0 _dynamicmaterial)
    (Audio|PlaySoundatLocation "/Game/PopFlow/Blueprints/FloatingBubblePuzzle/clank.clank" (Transformation|GetActorLocation) "0, 0, 0" 1.0 1.0 0.0 0 0 0 0)
    (CallFunction|PushSwitchDown)
    (switch Utilities|FlowControl|Switch|SwitchonE_FanMoveDirection (Variables|Default|GetSwitchType)
      (:NewEnumerator0
        (Default|MoveForward _fanref))
      (:NewEnumerator1
        (Default|MoveBack _fanref))
      (:NewEnumerator2
        (Default|TurnonFan _fanref)))))

(event OnComponentEndOverlap(Box)
  (params (OverlappedComponent :type Primitive%20Component%20Object%20Reference) (OtherActor :type Actor%20Object%20Reference) (OtherComp :type Primitive%20Component%20Object%20Reference) (OtherBodyIndex :type Integer))
  (bind _fanref (Variables|Default|GetFanRef))
  (bind _dynamicmaterial (Variables|Default|GetDynamicMaterial))
  (if (not (Variables|Default|GetbClonePlaced))
    (Rendering|Material|SetScalarParameterValue _dynamicmaterial "SwitchIntensity" 0.0 :!class /Script/Engine.MaterialInstanceDynamic)
    (Rendering|Material|SetMaterial (Variables|Default|GetSM_Temple_Floor_Tile_2m_01) 0 _dynamicmaterial)
    (CallFunction|PullSwitchUp)
    (switch Utilities|FlowControl|Switch|SwitchonE_FanMoveDirection (Variables|Default|GetSwitchType)
      (:NewEnumerator0
        (Default|StopMoving _fanref :!label _label))
      (:NewEnumerator1
        (goto _label))
      (:NewEnumerator2
        (Default|TurnOffFan _fanref)))))

(event Custom|PushSwitchDown
  (bind _alpha (Timeline|Move PlayFromStart)
    (:Update
      (Transformation|SetRelativeLocation (Variables|Default|GetSM_Temple_Floor_Tile_2m_01) (Math|Vector|Lerp(Vector) "0, 0, 0" "0.000000,0.000000,-20.000000" _alpha) false false))))

(event Custom|PullSwitchUp
  (bind _alpha (Timeline|Move ReverseFromEnd)
    (:Update
      (Transformation|SetRelativeLocation (Variables|Default|GetSM_Temple_Floor_Tile_2m_01) (Math|Vector|Lerp(Vector) "0, 0, 0" "0.000000,0.000000,-20.000000" _alpha) false false))))

(event Custom|SwitchOff
  (bind _fanref (Variables|Default|GetFanRef))
  (bind _dynamicmaterial (Variables|Default|GetDynamicMaterial))
  (if (not (Variables|Default|GetbClonePlaced))
    (Rendering|Material|SetScalarParameterValue _dynamicmaterial "SwitchIntensity" 0.0 :!class /Script/Engine.MaterialInstanceDynamic)
    (Rendering|Material|SetMaterial (Variables|Default|GetSM_Temple_Floor_Tile_2m_01) 0 _dynamicmaterial)
    (CallFunction|PullSwitchUp)
    (switch Utilities|FlowControl|Switch|SwitchonE_FanMoveDirection (Variables|Default|GetSwitchType)
      (:NewEnumerator0
        (Default|StopMoving _fanref :!label _label))
      (:NewEnumerator1
        (goto _label))
      (:NewEnumerator2
        (Default|TurnOffFan _fanref)))))

(event EventBeginPlay
  (bind _returnvalue (Rendering|Material|CreateDynamicMaterialInstance (Variables|Default|GetSM_Temple_Floor_Tile_2m_01) 0 "/Game/PopFlow/Blueprints/Materials/M_SwitchOn.M_SwitchOn" "None" :!class /Script/Engine.PrimitiveComponent))
  (Variables|Default|SetDynamicMaterial _returnvalue))

(fn ConstructionScript)