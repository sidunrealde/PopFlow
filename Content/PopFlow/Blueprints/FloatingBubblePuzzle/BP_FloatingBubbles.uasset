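; BP_FloatingBubbles is a bubble actor for the floating bubble puzzle that pops when destroyed.
; Its DestroyBubble event activates the PSNWaterHeavySurface particle, removes the mesh, calls the OnBubbleDestroyed dispatcher and plays a pop sound at its location.
; The actor destroys itself after a short delay, and a second delayed destroy chain is left unconnected.
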(event Custom|DestroyBubble
  (Components|Activation|Activate (Variables|Default|GetPSN_WaterHeavy_Surface) false)
  (Components|DestroyComponent (Variables|Default|GetStaticMesh))
  (Default|CallOnBubbleDestroyed)
  (Audio|PlaySoundatLocation "/Game/Interface_And_Item_Sounds/Cues/Abstract_Pop_02_Cue.Abstract_Pop_02_Cue" (Transformation|GetActorLocation) "0, 0, 0" 1.0 1.0 0.0 0 0 0 0)
  (Utilities|FlowControl|Delay 0.5)
  (Actor|DestroyActor))

(fn ConstructionScript)