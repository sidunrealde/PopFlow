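; BPP_MovingPlatform02 is a platform Blueprint that starts moving along a spline on BeginPlay, with an attached wind sound.
; A timeline's normalized distance, scaled by spline length, sets the Scene component's world location without sweep.
; The construction script sets the timeline's play rate from Speed.
; MoveReverse is empty and the timer that would call RunAfterDelay to alternate direction never runs, leaving that reversal logic inactive.
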(event Custom|StartMoving
  (bind _spline (Variables|Default|GetSpline))
  (bind (_direction _distancenormalized) (Timeline|Timeline PlayFromStart)
    (:Update
      (Transformation|SetWorldLocation (Variables|Default|GetScene) (Spline|GetLocationatDistanceAlongSpline _spline (* _distancenormalized (Spline|GetSplineLength _spline)) "World") false false))))

(event Custom|MoveReverse)

(event Custom|RunAfterDelay
  (switch Utilities|FlowControl|Switch|SwitchonETimelineDirection (stale Custom|StartMoving _direction)
    (:Forward
      (CallFunction|MoveReverse))
    (:Backward
      (CallFunction|StartMoving))))

(event EventBeginPlay
  (CallFunction|StartMoving)
  (Audio|SpawnSoundAttached "/Game/SmallSoundKit/SSKWav/AmbienceWav/Amb_Wind.Amb_Wind" (Variables|Default|GetScene) "None" "0, 0, 0" "0, 0, 0" "KeepRelativeOffset" false 1.0 1.0 0.0 0 0))

(event Collision|EventActorBeginOverlap
  (params (OtherActor :type Actor%20Object%20Reference)))

(event EventTick
  (params (DeltaSeconds :type Float%20%28single-precision%29)))

(fn ConstructionScript
  (Components|Timeline|SetPlayRate (Variables|Default|GetTimeline) (Variables|Default|GetSpeed)))