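; Moving platform that begins shuttling along a spline once its referenced activation bubble is popped.
; Construction parks the moving Scene component at the spline's end and applies Speed as the Move timeline's play rate.
; Popping spawns an attached rune sphere in the bubble's color, plays wind sound and starts reverse travel after a short delay.
; The timeline drives position by normalized spline distance, pausing after each run before flipping direction.
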(event Custom|OnBubblePopped_Event
  (params (Color :type E_BubbleColor%20Enum :default "NewEnumerator0"))
  (bind _returnvalue (Game|SpawnActorfromClass "/Game/Isometric_World/Sky_Temple/Blueprints/Runes/BP_Rune_Sphere_Circle_01.BP_Rune_Sphere_Circle_01_C" (Math|Transform|MakeTransform "0, 0, 0" "0, 0, 0" "1.000000,1.000000,1.000000") "Undefined" "MultiplyWithRoot" 0 0))
  (Transformation|AttachComponentToComponent _returnvalue (Variables|Default|GetAttachComponent) "None" "SnapToTarget" "SnapToTarget" "SnapToTarget" true)
  (Default|Activate _returnvalue Color)
  (Utilities|Time|SetTimerbyEvent (delegate Custom|MoveReverse) 1.0)
  (Audio|SpawnSoundAttached "/Game/PopFlow/Blueprints/FloatingBubblePuzzle/wind.wind" (Variables|Default|GetScene) "None" "0, 0, 0" "0, 0, 0" "KeepRelativeOffset" false 1.0 1.0 0.0 0 0))

(event Custom|StartMoving
  (bind _spline (Variables|Default|GetSpline))
  (bind (_direction _distancenormalized) (Timeline|Move PlayFromStart)
    (:Update
      (Transformation|SetWorldLocation (Variables|Default|GetScene) (Spline|GetLocationatDistanceAlongSpline _spline (* _distancenormalized (Spline|GetSplineLength _spline)) "World") false false))
    (:Finished
      (Utilities|Time|SetTimerbyEvent (delegate Custom|RunAfterDelay) 3.5))))

(event Custom|MoveReverse
  (bind _spline (Variables|Default|GetSpline))
  (bind (_direction _distancenormalized) (Timeline|Move ReverseFromEnd)
    (:Update
      (Transformation|SetWorldLocation (Variables|Default|GetScene) (Spline|GetLocationatDistanceAlongSpline _spline (* _distancenormalized (Spline|GetSplineLength _spline)) "World") false false))
    (:Finished
      (Utilities|Time|SetTimerbyEvent (delegate Custom|RunAfterDelay) 3.5))))

(event Custom|RunAfterDelay
  (switch Utilities|FlowControl|Switch|SwitchonETimelineDirection (stale Custom|StartMoving _direction)
    (:Forward
      (CallFunction|MoveReverse))
    (:Backward
      (CallFunction|StartMoving))))

(event EventBeginPlay
  (EventDispatchers|AssignOnBubblePopped (Variables|Default|GetActivationBubbleRef) (delegate Custom|OnBubblePopped_Event)))

(fn ConstructionScript
  (bind _spline (Variables|Default|GetSpline))
  (Components|Timeline|SetPlayRate (Variables|Default|GetMove) (Variables|Default|GetSpeed))
  (Transformation|SetWorldLocation (Variables|Default|GetScene) (Spline|GetLocationatDistanceAlongSpline _spline (Spline|GetSplineLength _spline) "World") false false))