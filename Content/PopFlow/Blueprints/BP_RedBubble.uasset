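; BP_RedBubble is a poppable bubble actor for PopFlow whose material follows its BubbleColor, despite the red name.
; Key bubbles also show a key mesh, bobbed by a ping-ponging Timeline.
; Character overlap plays pop sound and particles, broadcasts OnBubblePopped with the color and removes the mesh.
; It destroys itself after a short delay; key bubbles first add a key to ALS_GameMode_SP and play a chime.
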(event OnComponentBeginOverlap(StaticMesh)
  (params (OverlappedComponent :type Primitive%20Component%20Object%20Reference) (OtherActor :type Actor%20Object%20Reference) (OtherComp :type Primitive%20Component%20Object%20Reference) (OtherBodyIndex :type Integer) (bFromSweep :type Boolean) (SweepResult :type Hit%20Result%20Structure%20%28by%20ref%29))
  (Utilities|Casting|CastToCharacter OtherActor)
  (Audio|PlaySoundatLocation "/Game/Interface_And_Item_Sounds/Cues/Abstract_Pop_02_Cue.Abstract_Pop_02_Cue" (Transformation|GetActorLocation) "0, 0, 0" 1.0 1.0 0.0 0 0 0 0)
  (Components|Activation|Activate (Variables|Default|GetPSN_WaterHeavy_Surface) false)
  (Default|CallOnBubblePopped (Variables|Default|GetBubbleColor))
  (Components|DestroyComponent (Variables|Default|GetStaticMesh))
  (if (Variables|Default|GetbIsKey)
    (bind _asals_game_mode_sp (Utilities|Casting|CastToALS_GameMode_SP (Game|GetGameMode)))
    (Default|Addkey _asals_game_mode_sp)
    (Utilities|FlowControl|Delay 1.0)
    (Audio|PlaySoundatLocation "/Game/Interface_And_Item_Sounds/Cues/Special_Musical_03_Cue.Special_Musical_03_Cue" (Transformation|GetActorLocation) "0, 0, 0" 1.0 1.0 0.0 0 0 0 0)
    (Actor|DestroyActor)
    (else
      (Utilities|FlowControl|Delay 1.0)
      (Actor|DestroyActor))))

(event Custom|PlayForward
  (bind _keylocation (Variables|Default|GetKeylocation))
  (bind (_direction _newtrack_0) (Timeline|Timeline PlayFromStart)
    (:Update
      (Transformation|SetRelativeLocation (Variables|Default|GetKey) (Math|Vector|Lerp(Vector) (+ _keylocation "0.000000,0.000000,-3.000000") (+ _keylocation "0.000000,0.000000,3.000000") _newtrack_0) false false))
    (:Finished
      (switch Utilities|FlowControl|Switch|SwitchonETimelineDirection _direction
        (:Forward
          (CallFunction|PlayReverse))
        (:Backward
          (CallFunction|PlayForward))))))

(event Custom|PlayReverse
  (bind _keylocation (Variables|Default|GetKeylocation))
  (bind (_direction _newtrack_0) (Timeline|Timeline ReverseFromEnd)
    (:Update
      (Transformation|SetRelativeLocation (Variables|Default|GetKey) (Math|Vector|Lerp(Vector) (+ _keylocation "0.000000,0.000000,-3.000000") (+ _keylocation "0.000000,0.000000,3.000000") _newtrack_0) false false))
    (:Finished
      (switch Utilities|FlowControl|Switch|SwitchonETimelineDirection _direction
        (:Forward
          (CallFunction|PlayReverse))
        (:Backward
          (CallFunction|PlayForward))))))

(event EventBeginPlay
  (Variables|Default|SetKeylocation (Variables|/Script/Engine.SceneComponent|GetRelativeLocation (Variables|Default|GetKey)))
  (Rendering|Material|SetMaterial (Variables|Default|GetStaticMesh) 0 (Utilities|Select :Index (Variables|Default|GetBubbleColor) :NewEnumerator0 "/Game/PopFlow/Materials/RedBubble.RedBubble" :NewEnumerator1 "/Game/PopFlow/Materials/MI_BlueBubble.MI_BlueBubble" :NewEnumerator2 "/Game/PopFlow/Materials/MI_GreenBubble.MI_GreenBubble" :NewEnumerator3 "/Game/PopFlow/Materials/MI_KeyBubble.MI_KeyBubble"))
  (if (Variables|Default|GetbIsKey)
    (Components|StaticMesh|SetStaticMesh (Variables|Default|GetKey) (Variables|Default|GetKeyMesh))
    (CallFunction|PlayForward)))

(fn ConstructionScript)