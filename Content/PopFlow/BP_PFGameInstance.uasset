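; Game instance for PopFlow that shows the main menu and stores the player's character selection.
; CreateMainMenu creates the menu widget once, adds it to the viewport, switches to UI-only input with cursor, and binds four bubble buttons.
; Each button passes an index to SetCharacter, which stores the matching mesh and anim class from parallel arrays.
; It applies only the mesh to the BP_UICharacter found in the level.
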(event Custom|CreateMainMenu
  (bind _returnvalue (Game|GetPlayerController 0))
  (Variables|Default|GetMainMenuRef
    (:then
      _)
    (:else
      (bind _returnvalue_2 (UserInterface|CreateWidget "/Game/PopFlow/Assets/UI/W_MainMenu.W_MainMenu_C" (Game|GetPlayerController 0)))
      (Variables|Default|SetMainMenuRef _returnvalue_2)))
  (UserInterface|Viewport|AddtoViewport (Variables|Default|GetMainMenuRef) 0)
  (Input|SetInputModeUIOnly _returnvalue (Variables|Default|GetMainMenuRef) "DoNotLock" false)
  (Variables|/Script/Engine.PlayerController|SetbShowMouseCursor _returnvalue true)
  (EventDispatchers|AssignOnButtonClicked (Variables|/Game/PopFlow/Assets/UI/W_MainMenu.W_MainMenu_C|GetWBP_Bubbles01 (Variables|Default|GetMainMenuRef)) (delegate Custom|Bubbles01))
  (EventDispatchers|AssignOnButtonClicked (Variables|/Game/PopFlow/Assets/UI/W_MainMenu.W_MainMenu_C|GetWBP_Bubbles02 (Variables|Default|GetMainMenuRef)) (delegate Custom|Bubbles02))
  (EventDispatchers|AssignOnButtonClicked (Variables|/Game/PopFlow/Assets/UI/W_MainMenu.W_MainMenu_C|GetWBP_Bubbles03 (Variables|Default|GetMainMenuRef)) (delegate Custom|Bubbles03))
  (EventDispatchers|AssignOnButtonClicked (Variables|/Game/PopFlow/Assets/UI/W_MainMenu.W_MainMenu_C|GetWBP_Bubbles04 (Variables|Default|GetMainMenuRef)) (delegate Custom|Bubbles04)))

(event Custom|Bubbles01
  (CallFunction|SetCharacter))

(event Custom|Bubbles02
  (CallFunction|SetCharacter 1))

(event Custom|Bubbles03
  (CallFunction|SetCharacter 2))

(event Custom|Bubbles04
  (CallFunction|SetCharacter 3))

(fn SetCharacter
  (params (Dimension%201 :type Integer))
  (Variables|Default|SetSelectedMesh (Utilities|Array|Get(acopy) (Variables|Default|GetMeshArray) Dimension%201))
  (Variables|Default|SetSelectedAnimBP (Utilities|Array|Get(acopy) (Variables|Default|GetAnimInstanceArray) Dimension%201))
  (bind _returnvalue (Actor|GetActorOfClass "/Game/PopFlow/Assets/UI/BP_UICharacter.BP_UICharacter_C"))
  (Components|SkeletalMesh|SetSkeletalMeshAsset (Variables|/Game/PopFlow/Assets/UI/BP_UICharacter.BP_UICharacter_C|GetMesh _returnvalue) (Variables|Default|GetSelectedMesh)))